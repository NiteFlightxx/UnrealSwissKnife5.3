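; BP_Vol_Painter is an actor that paints density into a volume render target while the left mouse button is held.
; Each tick it projects a point along its forward vector into the referenced Mesh's local box, with debug guides; this update runs only when ShowCuides is on.
; Valid points drive a dynamic M_Vol_Painter material's sphere center, radius and density, drawn to the render target via canvas; ResetRT clears it.
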(event EventBeginPlay
  (bind _returnvalue (Rendering|Material|CreateDynamicMaterialInstance "/UnrealSwissKnife/HLSL/RayMarch/M_Vol_Painter.M_Vol_Painter" "None" "None" :!class /Script/Engine.KismetMaterialLibrary))
  (Variables|Default|SetDMI_VolPainter _returnvalue))

(event Collision|EventActorBeginOverlap
  (params (OtherActor :type Actor%20Object%20Reference)))

(event EventTick
  (params (DeltaSeconds :type Float%20%28single-precision%29))
  (CallFunction|UpdateTraces)
  (if (Variables|Default|GetIsPainting)
    (CallFunction|PaintVolume)))

(event Input|MouseEvents|DebugKeyLeftMouseButton
  (params (Key :type Key%20Structure :default "None") (ActionValue :type Input%20Action%20Value%20Structure))
  (:Pressed
    (Variables|Default|SetIsPainting true))
  (:Released
    (Variables|Default|SetIsPainting false)))

(fn ConstructionScript)

(fn PaintVolume
  (bind _dmi_volpainter (Variables|Default|GetDMI_VolPainter))
  (if (Variables|Default|GetValidPaintPosition)
    (bind (_canvas _size _context) (Rendering|BeginDrawCanvastoRenderTarget (Variables|Default|GetTexture%20Render%20Target)))
    (Rendering|Material|SetVectorParameterValue _dmi_volpainter "SphereCenter" (Math|Conversions|ToLinearColor(Vector) (Variables|Default|GetPaintPosition)) :!class /Script/Engine.MaterialInstanceDynamic)
    (Rendering|Material|SetScalarParameterValue _dmi_volpainter "Density" (Variables|Default|GetPaintDensity) :!class /Script/Engine.MaterialInstanceDynamic)
    (Rendering|Material|SetScalarParameterValue _dmi_volpainter "Radius" (/ (Variables|Default|GetPaintRadius) (.X (Math|Vector|BreakVector (Transformation|GetActorScale3D (Variables|Default|GetMesh))))) :!class /Script/Engine.MaterialInstanceDynamic)
    (Canvas|DrawMaterial :self _canvas :RenderMaterial _dmi_volpainter :ScreenSize _size :CoordinateSize "(X=1.000000,Y=1.000000)" :PivotPoint "(X=0.500000,Y=0.500000)")
    (Rendering|EndDrawCanvastoRenderTarget _context)))

(fn ResetRT
  (Rendering|ClearRenderTarget2D (Variables|Default|GetTexture%20Render%20Target)))

(fn UpdateTraces
  (bind _returnvalue (Transformation|GetActorLocation))
  (bind _returnvalue_2 (Transformation|GetActorForwardVector))
  (bind _mesh (Variables|Default|GetMesh))
  (bind _tracedistance (Variables|Default|GetTraceDistance))
  (bind _returnvalue_3 (Transformation|GetActorTransform _mesh))
  (bind _returnvalue_4 (* _returnvalue_2 _tracedistance))
  (bind _returnvalue_5 (+ _returnvalue _returnvalue_4))
  (bind _returnvalue_6 (Math|Transform|InverseTransformLocation _returnvalue_3 _returnvalue_5))
  (if (Variables|Default|GetShowCuides)
    (Rendering|Debug|DrawDebugBox (Transformation|GetActorLocation _mesh) (* (Transformation|GetActorScale3D _mesh) 5e+01) "(R=1.000000,G=0.000000,B=0.000000,A=1.000000)" (Transformation|GetActorRotation _mesh) 0.0 2.0)
    (bind _output_get (Variables|Default|SetValidPaintPosition (Class|GeometryScriptLibraryBoxFunctions|TestPointInsideBox (Class|GeometryScriptLibraryBoxFunctions|MakeBoxfromCenterExtents "0, 0, 0" "50.000000,50.000000,50.000000") _returnvalue_6 true)))
    (if _output_get
      _
      (else
        _))
    (Rendering|Debug|DrawDebugSphere _returnvalue_5 (* (Variables|Default|GetPaintRadius) 5e+01) 12 "(R=0.000000,G=1.000000,B=0.000000,A=1.000000)" 0.0)
    (Variables|Default|SetPaintPosition (/ _returnvalue_6 5e+01))))